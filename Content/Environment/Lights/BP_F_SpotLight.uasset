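; Spot light fixture Blueprint that supplies its two point light components to a parent class.
; On BeginPlay it clears the LightReference array and adds PointLight and PointLight1 before calling the parent BeginPlay.
; Tick and the construction script only forward to the parent, so any further behavior is inherited.
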(event `self.ReceiveBeginPlay`
  (bind _lightreference (`self.LightReference`))
  (`KismetArrayLibrary.Array_Clear` _lightreference)
  (`KismetArrayLibrary.Array_Add` _lightreference (`self.PointLight`))
  (`KismetArrayLibrary.Array_Add` _lightreference (`self.PointLight1`))
  (`parent.ReceiveBeginPlay`))

(event `self.ReceiveActorBeginOverlap`
  (params (OtherActor :type "Actor Object Reference")))

(event `self.ReceiveTick`
  (params (DeltaSeconds :type "Float (single-precision)"))
  (`parent.ReceiveTick` DeltaSeconds))

(fn `UserConstructionScript`
  (`parent.UserConstructionScript`))