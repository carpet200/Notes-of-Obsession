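; Template Blueprint for environment lights, deriving its behavior from a parent class.
; On BeginPlay it clears LightReference, refills it with its PointLight and SpotLight, then calls the parent BeginPlay.
; A "Delete unwanted" note marks the light entries as ones to trim in lights built from the template.
; Tick and the construction script only call the parent.
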(event `self.ReceiveBeginPlay`
  (bind _lightreference (`self.LightReference`))
  (`KismetArrayLibrary.Array_Clear` _lightreference)
  ;[1 1 1] Delete unwanted
  (`KismetArrayLibrary.Array_Add` _lightreference (`self.PointLight`))
  (`KismetArrayLibrary.Array_Add` (`self.LightReference`) (`self.SpotLight`))
  (`parent.ReceiveBeginPlay`))

(event `self.ReceiveActorBeginOverlap`
  (params (OtherActor :type "Actor Object Reference")))

(event `self.ReceiveTick`
  (params (DeltaSeconds :type "Float (single-precision)"))
  (`parent.ReceiveTick` DeltaSeconds))

(fn `UserConstructionScript`
  (`parent.UserConstructionScript`))