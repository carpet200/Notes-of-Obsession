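; Spook event: an elephant head that turns relative to the player's camera while the player is not looking.
; Entering the trigger box starts a short Delay polling loop until ProjectWorldToScreen fails for the head's location.
; It then destroys the box, making the scare one-shot, and snaps the head using the camera-to-head look-at with pitch zeroed and a 90-degree offset.
; The construction script places the box from the BoxTransform variable.
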(event `self.Box.OnComponentBeginOverlap`
  (params (OtherActor :type "Actor Object Reference") (OtherComp :type "PrimitiveComponent Object Reference") (OtherBodyIndex :type Integer) (bFromSweep :type Boolean) (SweepResult :type "HitResult Structure (by ref)"))
  (bind _head (`self.Head`))
  (if (not (`.ReturnValue` (`GameplayStatics.ProjectWorldToScreen` (`GameplayStatics.GetPlayerController` 0) (`SceneComponent.K2_GetComponentLocation` _head)))) :!label _label
    (`ActorComponent.K2_DestroyComponent` (`self.Box`))
    (`SceneComponent.K2_SetWorldRotation` _head (`KismetMathLibrary.ComposeRotators` (`KismetMathLibrary.MakeRotator` (.roll (`KismetMathLibrary.FindLookAtRotation` (`SceneComponent.K2_GetComponentLocation` (`PlayerCameraManager.TransformComponent` (`GameplayStatics.GetPlayerCameraManager` 0))) (`SceneComponent.K2_GetComponentLocation` _head))) 0.0 (.yaw (`KismetMathLibrary.FindLookAtRotation` (`SceneComponent.K2_GetComponentLocation` (`PlayerCameraManager.TransformComponent` (`GameplayStatics.GetPlayerCameraManager` 0))) (`SceneComponent.K2_GetComponentLocation` _head)))) (struct :`Yaw` 90.0)) false true)
    (else
      (`KismetSystemLibrary.Delay` 0.1)
      (goto _label))))

(fn `UserConstructionScript`
  (`SceneComponent.K2_SetRelativeTransform` (`self.Box`) (`self.BoxTransform`) false false))