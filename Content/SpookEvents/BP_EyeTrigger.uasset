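; Spook event trigger volume that re-aims a pair of eyes using the player's camera once both are on screen.
; Box overlap starts a 2.5-second delay, then polls every second until EyesInView passes or the overlap ends.
; EyesInView projects both eyes to screen space, then each eye rotates once along the camera-to-eye direction.
; The construction script places box and eyes from transform variables.
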(event `self.Box.OnComponentBeginOverlap`
  (params (OtherActor :type "Actor Object Reference") (OtherComp :type "PrimitiveComponent Object Reference") (OtherBodyIndex :type Integer) (bFromSweep :type Boolean) (SweepResult :type "HitResult Structure (by ref)"))
  (set `self.IsPlayerCurrent` true)
  (`KismetSystemLibrary.Delay` 2.5)
  (if (`self.IsPlayerCurrent`) :!label _label
    (bind _eyesinview (`self.EyesInView`))
    (if _eyesinview
      (bind _asbp_first_person_character_thereal (cast `/Game/Testing/BP_FirstPersonCharacter_THEREAL` (`GameplayStatics.GetPlayerCharacter` 0)))
      (bind _returnvalue (`SceneComponent.K2_GetComponentLocation` (`/Game/Testing/BP_FirstPersonCharacter_THEREAL.FirstPersonCamera` _asbp_first_person_character_thereal)))
      (`SceneComponent.K2_SetWorldRotation` (`self.Eye1`) (`KismetMathLibrary.FindLookAtRotation` _returnvalue (`SceneComponent.K2_GetComponentLocation` (`self.Eye1`))) false true)
      (`SceneComponent.K2_SetWorldRotation` (`self.Eye2`) (`KismetMathLibrary.FindLookAtRotation` _returnvalue (`SceneComponent.K2_GetComponentLocation` (`self.Eye2`))) false true)
      (else
        (`KismetSystemLibrary.Delay` 1.0)
        (goto _label)))))

(event `self.Box.OnComponentEndOverlap`
  (params (OtherActor :type "Actor Object Reference") (OtherComp :type "PrimitiveComponent Object Reference") (OtherBodyIndex :type Integer))
  (set `self.IsPlayerCurrent` false))

(fn `EyesInView`
  (returns (EyesInView :type Boolean))
  (bind (_x _y) (`KismetMathLibrary.BreakVector2D` (`WidgetLayoutLibrary.GetViewportSize`)))
  (bind (_screenposition _returnvalue) (`GameplayStatics.ProjectWorldToScreen` (`GameplayStatics.GetPlayerController` 0) (`SceneComponent.K2_GetComponentLocation` (`self.Eye2`))))
  (bind (_screenposition_2 _returnvalue_2) (`GameplayStatics.ProjectWorldToScreen` (`GameplayStatics.GetPlayerController` 0) (`SceneComponent.K2_GetComponentLocation` (`self.Eye1`))))
  (bind (_x_2 _y_2) (`KismetMathLibrary.BreakVector2D` _screenposition))
  (bind (_x_3 _y_3) (`KismetMathLibrary.BreakVector2D` _screenposition_2))
  (if _returnvalue_2
    (if _returnvalue
      (return (and (and (< _x_3 _x) (< _x_2 _x)) (and (< _y_3 _y) (< _y_2 _y))))
      (else
        _)))
  (return false))

(fn `UserConstructionScript`
  (`|ExecutionSequence`
    (:`then_0`
      (`SceneComponent.K2_SetRelativeTransform` (`self.Box`) (`self.CollisionTransform`) false false))
    (:`then_1`
      (`SceneComponent.K2_SetRelativeTransform` (`self.Eye1`) (`self.EyeTransform1`) false false))
    (:`then_2`
      (`SceneComponent.K2_SetRelativeTransform` (`self.Eye2`) (`self.EyeTransform2`) false false))))