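; BP_Plane is a plane actor among the spook events that drifts forward while flashing a white light.
; Each Tick offsets the root along its forward vector by one unit without sweeping, so its speed depends on frame rate.
; The blink comes from a real-time sine wave, clamped and rounded up into an on/off square wave that scales WhiteLightIntensity.
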(event `self.ReceiveBeginPlay`)

(event `self.ReceiveActorBeginOverlap`
  (params (OtherActor :type "Actor Object Reference")))

(event `self.ReceiveTick`
  (params (DeltaSeconds :type "Float (single-precision)"))
  (bind _defaultsceneroot (`self.DefaultSceneRoot`))
  (`LightComponent.SetIntensity` (`self.WhiteLight`) (* (`KismetMathLibrary.FCeil` (`KismetMathLibrary.FClamp` (`KismetMathLibrary.Sin` (/ (`GameplayStatics.GetRealTimeSeconds`) 0.1)))) (`self.WhiteLightIntensity`)))
  (`SceneComponent.K2_AddWorldOffset` _defaultsceneroot (`SceneComponent.GetForwardVector` _defaultsceneroot) false false))

(fn `UserConstructionScript`)