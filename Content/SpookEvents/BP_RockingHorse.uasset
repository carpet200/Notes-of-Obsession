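; Spook event rocking horse that starts rocking with sound when something first overlaps its one-shot Primer trigger, placed by an editable transform.
; The InitialPush timeline advances a sine phase and scales its amplitude by a falloff curve.
; CalculateRocking turns that value into pitch plus a compensating forward/back offset, starting from an editable angle.
; An attached audio event retriggers each positive half-swing, with volume following the falloff; the Tick looping branch is empty.
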(event `self.ReceiveTick`
  (params (DeltaSeconds :type "Float (single-precision)"))
  ;[1 1 1] Continue looping for eternity
  (if (stale `self.Primer.OnComponentBeginOverlap` _output_get_2)
    _))

(event `self.ReceiveBeginPlay`
  (bind _decal (`self.Decal`))
  (bind _decal_2 (`self.Decal`))
  ;[1 1 1] Get initial values
  (set `self.InitialPosition` (`SceneComponent.K2_GetComponentLocation` _decal_2))
  (set `self.InitialRotation` (`SceneComponent.K2_GetComponentRotation` _decal_2))
  (bind (_newrotation _newposition) (`self.CalculateRocking` (`KismetMathLibrary.Sin` (+ (stale `self.Primer.OnComponentBeginOverlap` _output_get) (/ (* (`self.StartAngle`) 3.1415) 180.0)))))
  (`SceneComponent.K2_SetWorldRotation` _decal _newrotation false true)
  (`SceneComponent.K2_SetWorldLocation` _decal _newposition false true))

(event `self.Primer.OnComponentBeginOverlap`
  (params (OtherActor :type "Actor Object Reference") (OtherComp :type "PrimitiveComponent Object Reference") (OtherBodyIndex :type Integer) (bFromSweep :type Boolean) (SweepResult :type "HitResult Structure (by ref)"))
  (bind _decal (`self.Decal`))
  (bind _returnvalue (`KismetMathLibrary.FClamp` (`self.RockingSpeed`) 0.0 1.0))
  ;[1 1 1] Normal rocking
  (`ActorComponent.K2_DestroyComponent` (`self.Primer`))
  (bind (_direction _rockingfalloff _rockingspeedfalloff) (`Timeline|InitialPush`)
    (:`Update`
      (set `self.RockingSpeed` _rockingfalloff)
      (bind _output_get (set `self.TickingTime` (+ (* _rockingspeedfalloff 2.5 (`GameplayStatics.GetWorldDeltaSeconds`)) (`self.TickingTime`))))
      (bind _returnvalue_2 (`KismetMathLibrary.Sin` (+ _output_get (/ (* (`self.StartAngle`) 3.1415) 180.0))))
      (bind (_newrotation _newposition) (`self.CalculateRocking` (* _returnvalue_2 _returnvalue)))
      ;[1 1 1] Sound control
      (`|ExecutionSequence`
        (:`then_0`
          (`SceneComponent.K2_SetWorldRotation` _decal _newrotation false true)
          (`SceneComponent.K2_SetWorldLocation` _decal _newposition false true))
        (:`then_1`
          (if (> _returnvalue_2 0.0)
            (`/Engine/EditorBlueprintResources/StandardMacros.DoOnce` false :!label _label
              (:`Completed`
                (bind _returnvalue_3 (`FMODBlueprintStatics.PlayEventAttached` "/Game/FMOD/Events/Ljud/Objects/Rocking_Elephant.Rocking_Elephant" (`self.fot_trappa1`) "None" (0.0 0.0 0.0) "KeepRelativeOffset"))))
            (else
              (goto _label :!via `Reset`)))))
      (`/Engine/EditorBlueprintResources/StandardMacros.IsValid` _returnvalue_3
        (:`Is Valid`
          (`FMODAudioComponent.SetVolume` _returnvalue_3 _returnvalue))))
    (:`Finished`
      ;[1 1 1] Continue looping for eternity
      (bind _output_get_2 (set `self.KeepLooping` true)))))

(fn `CalculateRocking`
  (params (RockingValue :type "Float (double-precision)"))
  (returns (NewRotation :type "Rotator Structure") (NewPosition :type "Vector Structure"))
  (bind _rockingdegree (`self.RockingDegree`))
  (return (`KismetMathLibrary.MakeRotator` 0.0 (* RockingValue _rockingdegree) (.yaw (`self.InitialRotation`))) (+ (* (`SceneComponent.GetForwardVector` (`self.DefaultSceneRoot`)) (* RockingValue (* (/ (`KismetMathLibrary.VSize` (- (`SceneComponent.K2_GetComponentLocation` (`self.Decal`)) (`SceneComponent.K2_GetComponentLocation` (`self.BottomPos`)))) (/ (/ (.z (`SceneComponent.RelativeLocation` (`self.Decal`))) 2.0) _rockingdegree)) -1.0))) (`self.InitialPosition`))))

(fn `UserConstructionScript`
  (`SceneComponent.K2_SetRelativeTransform` (`self.Primer`) (`self.TriggerTransform`) false false))