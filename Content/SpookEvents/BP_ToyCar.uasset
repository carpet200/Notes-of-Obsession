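; BP_ToyCar is a spook-event toy car that drives along a route actor's spline with its lights on while a music box plays.
; BeginPlay creates a rewind-looping iTween spline move oriented to the path, then immediately pauses it and hides the headlights and rear lights.
; OnMusicBoxStart shows the lights and resumes the tween.
; OnMusicBoxEnd hides them and pauses it again.
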(event `self.ReceiveBeginPlay`
  (`|ExecutionSequence`
    (:`then_0`
      (bind _returnvalue (`iTween.ActorMoveToSplinePointFull` 0.0 "No Name" self (`/Game/SpookEvents/BP_ToyCarRoute.Spline` (`self.RouteActor`)) true true "none" false 0.0 "first" "seconds" 20.0 "linear" null 1.0 "rewind" 0 true "orientToPath" null 50.0))
      (bind _output_get (set `self.ITweenReference` _returnvalue))
      (`iTween.PauseTweeningByEventReference` _output_get))
    (:`then_1`
      (`SceneComponent.SetVisibility` (`self.LigthLeft`) false false :!label _label)
      (`SceneComponent.SetVisibility` (`self.SpotLightLeft`) false false)
      (`SceneComponent.SetVisibility` (`self.LigthRight`) false false)
      (`SceneComponent.SetVisibility` (`self.SpotLightRight`) false false)
      (`SceneComponent.SetVisibility` (`self.RearLightLeft`) false false)
      (`SceneComponent.SetVisibility` (`self.RearLightRight`) false false)
      (`iTween.PauseTweeningByEventReference` (`self.ITweenReference`)))))

(event `self.OnMusicBoxStart`
  (`SceneComponent.SetVisibility` (`self.LigthLeft`) true false)
  (`SceneComponent.SetVisibility` (`self.SpotLightLeft`) true false)
  (`SceneComponent.SetVisibility` (`self.LigthRight`) true false)
  (`SceneComponent.SetVisibility` (`self.SpotLightRight`) true false)
  (`SceneComponent.SetVisibility` (`self.RearLightLeft`) true false)
  (`SceneComponent.SetVisibility` (`self.RearLightRight`) true false)
  (`iTween.ResumeTweeningByEventReference` (`self.ITweenReference`)))

(event `self.OnMusicBoxEnd`
  (goto _label))

(fn `UserConstructionScript`
  (`parent.UserConstructionScript`))