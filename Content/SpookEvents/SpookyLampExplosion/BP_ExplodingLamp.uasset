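; BP_ExplodingLamp is a spook-event lamp whose bulb can explode with sound and sparks.
; BeginPlay creates an audio component for the bulb-breaking event attached to LampSound and keeps it for later use.
; ExplodeLamp plays that component, swaps the bulb material to an unlit one, spawns a spark emitter at the point light and destroys the light.
; Nothing in this Blueprint calls ExplodeLamp.
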(event `self.ReceiveBeginPlay`
  (bind _returnvalue (`FMODBlueprintStatics.PlayEventAttached` "/Game/FMOD/Events/Ljud/LightBulb_Breaking.LightBulb_Breaking" (`self.LampSound`) "None" (0.0 0.0 0.0) "KeepRelativeOffset" false false)))

(event `ExplodeLamp`
  (`FMODAudioComponent.Play` (stale `self.ReceiveBeginPlay` _returnvalue))
  (`PrimitiveComponent.SetMaterial` (`self.Mesh_WardrobeLight_01`) 1 "/Game/SpookEvents/SpookyLampExplosion/Lightbulb_off.Lightbulb_off")
  (`GameplayStatics.SpawnEmitterAtLocation` "/Game/SpookEvents/SpookyLampExplosion/Lightbulb_Sparks.Lightbulb_Sparks" (`SceneComponent.K2_GetComponentLocation` (`self.PointLight`)))
  (`ActorComponent.K2_DestroyComponent` (`self.PointLight`)))

(fn `UserConstructionScript`)