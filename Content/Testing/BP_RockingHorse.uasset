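; BP_RockingHorse is a spook prop that starts rocking when something overlaps its trigger box.
; The construction script places the box from TriggerTransform.
; Overlap plays a TriggerAnim timeline for the initial jolt, then a RockingAnim timeline for normal rocking.
; Both feed CalculateRocking, which converts the curve value into pitch plus a compensating offset along the root's forward axis, applied to the Decal component relative to its starting transform.
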(event `self.ReceiveBeginPlay`
  (bind _decal (`self.Decal`))
  ;[1 1 1] Get initial values
  (set `self.InitialPosition` (`SceneComponent.K2_GetComponentLocation` _decal))
  (set `self.InitialRotation` (`SceneComponent.K2_GetComponentRotation` _decal)))

(event `self.Box.OnComponentBeginOverlap`
  (params (OtherActor :type "Actor Object Reference") (OtherComp :type "PrimitiveComponent Object Reference") (OtherBodyIndex :type Integer) (bFromSweep :type Boolean) (SweepResult :type "HitResult Structure (by ref)"))
  (bind _decal (`self.Decal`))
  (bind _decal_2 (`self.Decal`))
  ;[1 1 1] Initial spook
  (bind (_direction _triggervalue) (`Timeline|TriggerAnim`)
    (:`Update`
      (bind (_newrotation _newposition) (`self.CalculateRocking` _triggervalue))
      (`SceneComponent.K2_SetWorldRotation` _decal _newrotation false true)
      (`SceneComponent.K2_SetWorldLocation` _decal _newposition false true))
    (:`Finished`
      ;[1 1 1] Normal rocking
      (bind (_direction_2 _spookvalue) (`Timeline|RockingAnim`)
        (:`Update`
          (bind (_newrotation_2 _newposition_2) (`self.CalculateRocking` _spookvalue))
          (`SceneComponent.K2_SetWorldRotation` _decal_2 _newrotation_2 false true)
          (`SceneComponent.K2_SetWorldLocation` _decal_2 _newposition_2 false true))))))

(fn `CalculateRocking`
  (params (RockingValue :type "Float (double-precision)"))
  (returns (NewRotation :type "Rotator Structure") (NewPosition :type "Vector Structure"))
  (bind _rockingdegree (`self.RockingDegree`))
  (return (`KismetMathLibrary.MakeRotator` 0.0 (* RockingValue _rockingdegree) (.yaw (`self.InitialRotation`))) (+ (* (`SceneComponent.GetForwardVector` (`self.DefaultSceneRoot`)) (* RockingValue (* (/ (`KismetMathLibrary.VSize` (- (`SceneComponent.K2_GetComponentLocation` (`self.Decal`)) (`SceneComponent.K2_GetComponentLocation` (`self.BottomPos`)))) (/ (/ (.z (`SceneComponent.RelativeLocation` (`self.Decal`))) 2.0) _rockingdegree)) -1.0))) (`self.InitialPosition`))))

(fn `UserConstructionScript`
  (`SceneComponent.K2_SetRelativeTransform` (`self.Box`) (`self.TriggerTransform`) false true))